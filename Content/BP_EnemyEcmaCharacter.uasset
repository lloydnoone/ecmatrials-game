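; BP_EnemyEcmaCharacter is an enemy character Blueprint that links itself to its health bar widget.
; On BeginPlay it runs the parent logic, gets the user widget from the HealthBar component, casts it to WBP_EnemyHealthBar and sets that widget's Enemy reference to itself.
; The construction script only calls the parent, and the overlap and Tick events are disabled.
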(event `self.ReceiveBeginPlay`
  (`parent.ReceiveBeginPlay`)
  ;[1 1 1] Set the enemy variable for the health bar
  (bind _aswbp_enemy_health_bar (cast `/Game/UI/WBP_EnemyHealthBar` (`WidgetComponent.GetUserWidgetObject` (`self.HealthBar`)))) ; convert to our type to get enemy variable in healthbarBP
  (set `/Game/UI/WBP_EnemyHealthBar.Enemy` self _aswbp_enemy_health_bar) ; attach to this enemy to healthbar reference
)

(fn `UserConstructionScript`
  (`parent.UserConstructionScript`))