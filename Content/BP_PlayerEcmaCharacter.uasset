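; Player character Blueprint that currently adds no working behavior of its own: Tick and the construction script only call their parents.
; Unconnected leftover logic shows click-through on 3D widgets via a WidgetInteraction component, giving keyboard focus to an access panel's text input.
; Another unconnected chain focuses the code input of an overlapped BP_AccessPanel.
; None of this logic runs, as BeginPlay is disabled and ActorBeginOverlap is empty.
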(event `Key|LeftControl`
  (params (Key :type "Key Structure")))

(event `self.ReceiveActorBeginOverlap`
  (params (OtherActor :type "Actor Object Reference")))

(event `self.ReceiveTick`
  (params (DeltaSeconds :type "Float (single-precision)"))
  (`parent.ReceiveTick` DeltaSeconds))

(event `Key|RightMouseButton`
  (params (Key :type "Key Structure"))
  ;[1 1 1] right click the 3d widget. Get keyboard focus.
)

(fn `UserConstructionScript`
  (`parent.UserConstructionScript`))