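; BP_MeleeBoss is the melee boss Blueprint for Etasphera22, with a body assembled from many separate skeletal mesh parts.
; Its construction script binds every arm, leg, finger, torso and head piece to the main Mesh through Set Master Pose Component.
; The segmented pieces therefore follow the pose of that one mesh, and the script contains no other logic.
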(fn `UserConstructionScript`
  (`SkinnedMeshComponent.SetLeaderPoseComponent` (`self.SK_Etasphera22_Arm_Leg_calf_r`) (`self.Mesh`) false)
  (`SkinnedMeshComponent.SetLeaderPoseComponent` (`self.SK_Etasphera22_Arm_Leg_foot_l`) (`self.Mesh`) false)
  (`SkinnedMeshComponent.SetLeaderPoseComponent` (`self.SK_Etasphera22_Arm_Leg_foot_r`) (`self.Mesh`) false)
  (`SkinnedMeshComponent.SetLeaderPoseComponent` (`self.SK_Etasphera22_Arm_leg_hand_l`) (`self.Mesh`) false)
  (`SkinnedMeshComponent.SetLeaderPoseComponent` (`self.SK_Etasphera22_Arm_leg_hand_r`) (`self.Mesh`) false)
  (`SkinnedMeshComponent.SetLeaderPoseComponent` (`self.SK_Etasphera22_Arm_Leg_calf_l`) (`self.Mesh`) false)
  (`SkinnedMeshComponent.SetLeaderPoseComponent` (`self.SK_Etasphera22_Arm_Leg_pinky_02_l`) (`self.Mesh`) false)
  (`SkinnedMeshComponent.SetLeaderPoseComponent` (`self.SK_Etasphera22_Arm_Leg_index_01_l`) (`self.Mesh`) false)
  (`SkinnedMeshComponent.SetLeaderPoseComponent` (`self.SK_Etasphera22_Arm_Leg_index_01_r`) (`self.Mesh`) false)
  (`SkinnedMeshComponent.SetLeaderPoseComponent` (`self.SK_Etasphera22_Arm_Leg_index_02_l`) (`self.Mesh`) false)
  (`SkinnedMeshComponent.SetLeaderPoseComponent` (`self.SK_Etasphera22_Arm_Leg_index_02_r`) (`self.Mesh`) false)
  (`SkinnedMeshComponent.SetLeaderPoseComponent` (`self.SK_Etasphera22_Arm_Leg_index_03_l`) (`self.Mesh`) false)
  (`SkinnedMeshComponent.SetLeaderPoseComponent` (`self.SK_Etasphera22_Arm_Leg_index_03_r`) (`self.Mesh`) false)
  (`SkinnedMeshComponent.SetLeaderPoseComponent` (`self.SK_Etasphera22_Arm_leg_lowerarm_l`) (`self.Mesh`) false)
  (`SkinnedMeshComponent.SetLeaderPoseComponent` (`self.SK_Etasphera22_Arm_leg_lowerarm_r`) (`self.Mesh`) false)
  (`SkinnedMeshComponent.SetLeaderPoseComponent` (`self.SK_Etasphera22_Arm_Leg_middle_01_l`) (`self.Mesh`) false)
  (`SkinnedMeshComponent.SetLeaderPoseComponent` (`self.SK_Etasphera22_Arm_Leg_middle_01_r`) (`self.Mesh`) false)
  (`SkinnedMeshComponent.SetLeaderPoseComponent` (`self.SK_Etasphera22_Arm_Leg_middle_02_l`) (`self.Mesh`) false)
  (`SkinnedMeshComponent.SetLeaderPoseComponent` (`self.SK_Etasphera22_Arm_Leg_middle_02_r`) (`self.Mesh`) false)
  (`SkinnedMeshComponent.SetLeaderPoseComponent` (`self.SK_Etasphera22_Arm_Leg_middle_03_l`) (`self.Mesh`) false)
  (`SkinnedMeshComponent.SetLeaderPoseComponent` (`self.SK_Etasphera22_Arm_Leg_middle_03_r`) (`self.Mesh`) false)
  (`SkinnedMeshComponent.SetLeaderPoseComponent` (`self.SK_Etasphera22_Arm_Leg_pinky_01_l`) (`self.Mesh`) false)
  (`SkinnedMeshComponent.SetLeaderPoseComponent` (`self.SK_Etasphera22_Arm_Leg_pinky_01_r`) (`self.Mesh`) false)
  (`SkinnedMeshComponent.SetLeaderPoseComponent` (`self.SK_Etasphera22_Arm_Leg_thumb_03_r`) (`self.Mesh`) false)
  (`SkinnedMeshComponent.SetLeaderPoseComponent` (`self.SK_Etasphera22_Arm_Leg_pinky_02_r`) (`self.Mesh`) false)
  (`SkinnedMeshComponent.SetLeaderPoseComponent` (`self.SK_Etasphera22_Arm_Leg_pinky_03_l`) (`self.Mesh`) false)
  (`SkinnedMeshComponent.SetLeaderPoseComponent` (`self.SK_Etasphera22_Arm_Leg_pinky_03_r`) (`self.Mesh`) false)
  (`SkinnedMeshComponent.SetLeaderPoseComponent` (`self.SK_Etasphera22_Arm_Leg_ring_01_l`) (`self.Mesh`) false)
  (`SkinnedMeshComponent.SetLeaderPoseComponent` (`self.SK_Etasphera22_Arm_Leg_ring_01_r`) (`self.Mesh`) false)
  (`SkinnedMeshComponent.SetLeaderPoseComponent` (`self.SK_Etasphera22_Arm_Leg_ring_02_l`) (`self.Mesh`) false)
  (`SkinnedMeshComponent.SetLeaderPoseComponent` (`self.SK_Etasphera22_Arm_Leg_ring_02_r`) (`self.Mesh`) false)
  (`SkinnedMeshComponent.SetLeaderPoseComponent` (`self.SK_Etasphera22_Arm_Leg_ring_03_l`) (`self.Mesh`) false)
  (`SkinnedMeshComponent.SetLeaderPoseComponent` (`self.SK_Etasphera22_Arm_Leg_ring_03_r`) (`self.Mesh`) false)
  (`SkinnedMeshComponent.SetLeaderPoseComponent` (`self.SK_Etasphera22_Arm_Leg_thigh_l`) (`self.Mesh`) false)
  (`SkinnedMeshComponent.SetLeaderPoseComponent` (`self.SK_Etasphera22_Arm_Leg_thigh_r`) (`self.Mesh`) false)
  (`SkinnedMeshComponent.SetLeaderPoseComponent` (`self.SK_Etasphera22_Arm_Leg_thumb_01_l`) (`self.Mesh`) false)
  (`SkinnedMeshComponent.SetLeaderPoseComponent` (`self.SK_Etasphera22_Arm_Leg_thumb_01_r`) (`self.Mesh`) false)
  (`SkinnedMeshComponent.SetLeaderPoseComponent` (`self.SK_Etasphera22_Arm_Leg_thumb_02_l`) (`self.Mesh`) false)
  (`SkinnedMeshComponent.SetLeaderPoseComponent` (`self.SK_Etasphera22_Arm_Leg_thumb_02_r`) (`self.Mesh`) false)
  (`SkinnedMeshComponent.SetLeaderPoseComponent` (`self.SK_Etasphera22_Arm_Leg_thumb_03_l`) (`self.Mesh`) false)
  (`SkinnedMeshComponent.SetLeaderPoseComponent` (`self.SK_Etasphera22_Arm_leg_upperarm_r`) (`self.Mesh`) false)
  (`SkinnedMeshComponent.SetLeaderPoseComponent` (`self.SK_Etasphera22_Arm_leg_upperarm_l`) (`self.Mesh`) false)
  (`SkinnedMeshComponent.SetLeaderPoseComponent` (`self.SK_Etasphera22_Body_clavicle_l`) (`self.Mesh`) false)
  (`SkinnedMeshComponent.SetLeaderPoseComponent` (`self.SK_Etasphera22_Body_clavicle_r`) (`self.Mesh`) false)
  (`SkinnedMeshComponent.SetLeaderPoseComponent` (`self.SK_Etasphera22_Body_Head`) (`self.Mesh`) false)
  (`SkinnedMeshComponent.SetLeaderPoseComponent` (`self.SK_Etasphera22_Body_hips`) (`self.Mesh`) false)
  (`SkinnedMeshComponent.SetLeaderPoseComponent` (`self.SK_Etasphera22_Body_spine1`) (`self.Mesh`) false)
  (`SkinnedMeshComponent.SetLeaderPoseComponent` (`self.SK_Etasphera22_Body_spine2`) (`self.Mesh`) false)
  (`SkinnedMeshComponent.SetLeaderPoseComponent` (`self.SK_Etasphera22_Body_spine3`) (`self.Mesh`) false))