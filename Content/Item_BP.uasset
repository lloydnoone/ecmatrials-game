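; Base pickup item Blueprint that EcmaCharacter collects by overlapping its Box component, staying collected through the game instance.
; On overlap it calls PickUp, which registers its ActorID as destroyed in BP_EcmaGameInstance, then destroys itself.
; Shortly after BeginPlay it asks the game instance whether that ID was already destroyed and removes itself if so, so collected items do not reappear.
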(event `self.Box.OnComponentBeginOverlap`
  (params (OverlappedComponent :type "PrimitiveComponent Object Reference") (OtherActor :type "Actor Object Reference") (OtherComp :type "PrimitiveComponent Object Reference") (OtherBodyIndex :type Integer) (bFromSweep :type Boolean) (SweepResult :type "HitResult Structure (by ref)"))
  (cast `EcmaCharacter` OtherActor)
  (`self.PickUp`)
  (`self.K2_DestroyActor`))

(event `self.ReceiveBeginPlay`
  (`KismetSystemLibrary.Delay` 0.2)
  (bind _asecma_game_instance (cast `/Game/BP_EcmaGameInstance` (`GameplayStatics.GetGameInstance`)))
  (bind _destroyedalready (`/Game/BP_EcmaGameInstance.CheckIfAlreadyDestroyed` _asecma_game_instance (`self.ActorID`)))
  (if _destroyedalready
    (`self.K2_DestroyActor`)))

(event `PickUp`
  (bind _asecma_game_instance (cast `/Game/BP_EcmaGameInstance` (`GameplayStatics.GetGameInstance`)))
  (`/Game/BP_EcmaGameInstance.DestroyPersistentItem` _asecma_game_instance (`self.ActorID`)))

(fn `UserConstructionScript`)